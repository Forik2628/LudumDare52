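; A trigger-activated camera actor that follows the player along a spline rail.
; Overlapping its Box, or BeginPlay when Active is set, makes it player 0's view target.
; Each Tick moves the CineCamera to the spline point closest to the player pawn, shifted along the spline direction by CameraDirectionOffset, and rotates it to look at the pawn.
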(event OnComponentBeginOverlap(Box)
  (params (OverlappedComponent :type Primitive%20Component%20Object%20Reference) (OtherActor :type Actor%20Object%20Reference) (OtherComp :type Primitive%20Component%20Object%20Reference) (OtherBodyIndex :type Integer) (bFromSweep :type Boolean) (SweepResult :type Hit%20Result%20Structure%20%28by%20ref%29))
  (Game|Player|SetViewTargetwithBlend (Game|GetPlayerController 0) self 0.0 "VTBlend_Linear" 0.0 false))

(event EventTick
  (params (DeltaSeconds :type Float%20%28single-precision%29))
  (bind _returnvalue (Game|Player|GetPlayerPawn 0))
  (bind _cameraspline (Variables|Default|GetCameraSpline))
  (bind _returnvalue_2 (Transformation|GetActorLocation _returnvalue))
  (Utilities|IsValid (Game|Player|GetPlayerPawn 0)
    (:Is%20Valid
      (Transformation|SetWorldLocation (Variables|Default|GetCineCamera) (+ (* (Spline|FindDirectionClosesttoWorldLocation _cameraspline _returnvalue_2 "World") (Variables|Default|GetCameraDirectionOffset)) (Spline|FindLocationClosesttoWorldLocation _cameraspline _returnvalue_2 "World")) false false)
      (Transformation|SetWorldRotation (Variables|Default|GetCineCamera) (Math|Rotator|FindLookatRotation (Transformation|GetWorldLocation (Variables|Default|GetCineCamera)) (Transformation|GetActorLocation (Game|Player|GetPlayerPawn 0))) false false))))

(event EventBeginPlay
  (if (Variables|Default|GetActive)
    (Game|Player|SetViewTargetwithBlend (Game|GetPlayerController 0) self 0.0 "VTBlend_Linear" 0.0 false)))

(fn ConstructionScript)