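; BP_WellSoul is a soul actor that flies a desert character skeletal mesh along a spline when SpawnSoul is called.
; BeginPlay sets the Timeline play rate to the inverse of SoulFlyPlayRate.
; Each Timeline update maps its track to spline distance and sets the mesh's world transform, taking location in world space but rotation in local space.
; Disconnected nodes, including randomized timing and initial placement, never run.
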(event Custom|SpawnSoul
  (bind _spline (Variables|Default|GetSpline))
  (bind _newtrack_0 (Timeline|Timeline PlayFromStart)
    (:Update
      (Transformation|SetWorldTransform (Variables|Default|GetSKM_DesertCharacter) (Math|Transform|MakeTransform (Spline|GetLocationatDistanceAlongSpline _spline (Math|Float|Lerp 0.0 (Spline|GetSplineLength (Variables|Default|GetSpline)) _newtrack_0) "World") (Spline|GetRotationatDistanceAlongSpline _spline (Math|Float|Lerp 0.0 (Spline|GetSplineLength (Variables|Default|GetSpline)) _newtrack_0) "Local") "1.000000,1.000000,1.000000") false false))))

(event EventBeginPlay
  (Components|Timeline|SetPlayRate (Variables|Default|GetTimeline) (/ 1.0 (Variables|Default|GetSoulFlyPlayRate))))

(fn ConstructionScript)