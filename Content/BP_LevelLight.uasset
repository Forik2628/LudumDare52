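; BP_LevelLight controls a directional light that temporarily swings to an "illusion lightning" rotation and back.
; IllusionLightningON plays a timeline that lerps the light's relative rotation from default to illusion.
; That timeline's "Change Sky Mat" event waits IllusionDelay, then calls IllusionLightninOFF, whose own timeline lerps the rotation back.
; Despite the event's name, no sky material is changed here.
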(event Custom|IllusionLightningON
  (bind _newtrack_0 (Timeline|Timeline PlayFromStart)
    (:Update
      (Transformation|SetRelativeRotation (Variables|Default|GetDirectionalLight) (Math|Rotator|Lerp(Rotator) (Variables|Default|GetDefaultLightRot) (Variables|Default|GetIllusionLightRot) _newtrack_0) false false))
    (:ChangeSkyMat
      (Utilities|FlowControl|Delay (Variables|Default|GetIllusionDelay))
      (CallFunction|IllusionLightninOFF))))

(event Custom|IllusionLightninOFF
  (bind _newtrack_0 (Timeline|Timeline_0 PlayFromStart)
    (:Update
      (Transformation|SetRelativeRotation (Variables|Default|GetDirectionalLight) (Math|Rotator|Lerp(Rotator) (Variables|Default|GetIllusionLightRot) (Variables|Default|GetDefaultLightRot) _newtrack_0) false false))))

(event EventBeginPlay)

(fn ConstructionScript)