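; Illusion zone that makes sets of level actors appear or disappear as illusion vision toggles.
; When the player enters TriggerRadius, it registers itself on the character and calls IllusionON, with a delayed DoOnce reset.
; VisionON and VisionOFF switch mesh collision between Block and Ignore on separate actor lists and build dynamic materials.
; Timelines animate their blend and emissive parameters, fading the Barrier out on VisionON and in on VisionOFF.
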(event OnComponentBeginOverlap(TriggerRadius)
  (params (OverlappedComponent :type Primitive%20Component%20Object%20Reference) (OtherActor :type Actor%20Object%20Reference) (OtherComp :type Primitive%20Component%20Object%20Reference) (OtherBodyIndex :type Integer) (bFromSweep :type Boolean) (SweepResult :type Hit%20Result%20Structure%20%28by%20ref%29))
  (bind _asbp_third_person_character (Utilities|Casting|CastToBP_ThirdPersonCharacter OtherActor))
  (Variables|Default|SetCharacterRef _asbp_third_person_character)
  (Utilities|FlowControl|DoOnce false :!label _label
    (:Completed
      (Variables|/Game/DesertCharacter/BP_ThirdPersonCharacter.BP_ThirdPersonCharacter_C|SetBP_IllusionRef (Variables|Default|GetCharacterRef) self)
      (Default|IllusionON (Variables|Default|GetCharacterRef))
      (Utilities|FlowControl|Delay (Variables|Default|GetDuration))
      (goto _label Reset))))

(event Custom|VisionON
  (bind _barrier (Variables|Default|GetBarrier))
  (Utilities|Array|Clear (Variables|Default|GetDissappearMaterials))
  (Utilities|Array|Clear (Variables|Default|GetAppearMaterials))
  (for _array_element (Variables|Default|GetIllusionOnAppearActors)
    (Collision|SetCollisionResponsetoAllChannels (Actor|GetComponentbyClass _array_element "/Script/Engine.StaticMeshComponent") "ECR_Block")
    (for _array_element_2 (Rendering|Material|GetMaterials (Actor|GetComponentbyClass _array_element "/Script/Engine.StaticMeshComponent"))
      (bind _returnvalue (Rendering|Material|CreateDynamicMaterialInstance (Actor|GetComponentbyClass _array_element "/Script/Engine.StaticMeshComponent") (Utilities|Array|Length (Variables|Default|GetAppearMaterials)) _array_element_2 "None" :!class /Script/Engine.PrimitiveComponent))
      (Utilities|Array|Add (Variables|Default|GetAppearMaterials) _returnvalue)))
  (for _array_element_3 (Variables|Default|GetIllusionOnDissappearActors)
    (Collision|SetCollisionResponsetoAllChannels (Actor|GetComponentbyClass _array_element_3 "/Script/Engine.StaticMeshComponent") "ECR_Ignore")
    (for _array_element_4 (Rendering|Material|GetMaterials (Actor|GetComponentbyClass _array_element_3 "/Script/Engine.StaticMeshComponent"))
      (bind _returnvalue_2 (Rendering|Material|CreateDynamicMaterialInstance (Actor|GetComponentbyClass _array_element_3 "/Script/Engine.StaticMeshComponent") (Utilities|Array|Length (Variables|Default|GetDissappearMaterials)) _array_element_4 "None" :!class /Script/Engine.PrimitiveComponent))
      (Utilities|Array|Add (Variables|Default|GetDissappearMaterials) _returnvalue_2)))
  (bind _returnvalue_3 (Rendering|Material|CreateDynamicMaterialInstance _barrier 0 (Rendering|Material|GetMaterial _barrier 0) "None" :!class /Script/Engine.PrimitiveComponent))
  (Utilities|Array|Add (Variables|Default|GetDissappearMaterials) _returnvalue_3)
  (CallFunction|MaterialAppear)
  (CallFunction|MaterialDissapear))

(event Custom|VisionOFF
  (bind _barrier (Variables|Default|GetBarrier))
  (Utilities|Array|Clear (Variables|Default|GetDissappearMaterials))
  (Utilities|Array|Clear (Variables|Default|GetAppearMaterials))
  (Utilities|FlowControl|Sequence
    (:then_0
      (for _array_element (Variables|Default|GetIllusionOffAppearActors)
        (Collision|SetCollisionResponsetoAllChannels (Actor|GetComponentbyClass _array_element "/Script/Engine.StaticMeshComponent") "ECR_Block")
        (for _array_element_2 (Rendering|Material|GetMaterials (Actor|GetComponentbyClass _array_element "/Script/Engine.StaticMeshComponent"))
          (bind _returnvalue (Rendering|Material|CreateDynamicMaterialInstance (Actor|GetComponentbyClass _array_element "/Script/Engine.StaticMeshComponent") (Utilities|Array|Length (Variables|Default|GetAppearMaterials)) _array_element_2 "None" :!class /Script/Engine.PrimitiveComponent))
          (Utilities|Array|Add (Variables|Default|GetAppearMaterials) _returnvalue)))
      (for _array_element_3 (Variables|Default|GetIllusionOffDissappearActors)
        (Collision|SetCollisionResponsetoAllChannels (Actor|GetComponentbyClass _array_element_3 "/Script/Engine.StaticMeshComponent") "ECR_Ignore")
        (for _array_element_4 (Rendering|Material|GetMaterials (Actor|GetComponentbyClass _array_element_3 "/Script/Engine.StaticMeshComponent"))
          (bind _returnvalue_2 (Rendering|Material|CreateDynamicMaterialInstance (Actor|GetComponentbyClass _array_element_3 "/Script/Engine.StaticMeshComponent") (Utilities|Array|Length (Variables|Default|GetDissappearMaterials)) _array_element_4 "None" :!class /Script/Engine.PrimitiveComponent))
          (Utilities|Array|Add (Variables|Default|GetDissappearMaterials) _returnvalue_2))))
    (:then_1
      (bind _returnvalue_3 (Rendering|Material|CreateDynamicMaterialInstance _barrier 0 (Rendering|Material|GetMaterial _barrier 0) "None" :!class /Script/Engine.PrimitiveComponent))
      (Utilities|Array|Add (Variables|Default|GetAppearMaterials) _returnvalue_3)
      (CallFunction|MaterialAppear)
      (CallFunction|MaterialDissapear))))

(event Custom|MaterialDissapear
  (bind (_direction _newtrack_0 _newtrack_2) (Timeline|Timeline PlayFromStart)
    (:Update
      (for _array_element (Variables|Default|GetDissappearMaterials)
        (Rendering|Material|SetScalarParameterValue _array_element "AppearanceBlend" _newtrack_0 :!class /Script/Engine.MaterialInstanceDynamic)
        (Rendering|Material|SetScalarParameterValue _array_element "Emissive_Mult" _newtrack_2 :!class /Script/Engine.MaterialInstanceDynamic)))))

(event Custom|MaterialAppear
  (bind (_direction _newtrack_0 _newtrack_1) (Timeline|Timeline_0 PlayFromStart)
    (:Update
      (for _array_element (Variables|Default|GetAppearMaterials)
        (Rendering|Material|SetScalarParameterValue _array_element "AppearanceBlend" _newtrack_0 :!class /Script/Engine.MaterialInstanceDynamic)
        (Rendering|Material|SetScalarParameterValue _array_element "Emissive_Mult" _newtrack_1 :!class /Script/Engine.MaterialInstanceDynamic)))))

(event EventBeginPlay
  (bind _returnvalue (Actor|GetActorOfClass "/Game/DesertCharacter/BP_ThirdPersonCharacter.BP_ThirdPersonCharacter_C"))
  (bind _output_get (Variables|Default|SetCharacterRef _returnvalue))
  (Components|Timeline|SetPlayRate (Variables|Default|GetTimeline) (Variables|/Game/DesertCharacter/BP_ThirdPersonCharacter.BP_ThirdPersonCharacter_C|GetTimelinePlayrates _output_get)))

(fn ConstructionScript)