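; Final illusion area actor that toggles vision-dependent geometry and plays the game's ending cinematic.
; VisionON/VisionOFF swap collision on actor lists and fade them and the Barrier through dynamic material timelines.
; Overlapping the Box once starts camera cuts, a spline walk, a lerped fall, a mesh swap and a spline flight with lens changes, then quits.
; Its CineCamera tracks the player on Tick; TestLastScene jumps straight to the sequence.
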(event OnComponentBeginOverlap(Box)
  (params (OverlappedComponent :type Primitive%20Component%20Object%20Reference) (OtherActor :type Actor%20Object%20Reference) (OtherComp :type Primitive%20Component%20Object%20Reference) (OtherBodyIndex :type Integer) (bFromSweep :type Boolean) (SweepResult :type Hit%20Result%20Structure%20%28by%20ref%29))
  (bind _returnvalue (Game|GetPlayerCharacter 0))
  (bind _returnvalue_2 (Game|GetPlayerCharacter 0))
  (bind _flyspline (Variables|Default|GetFlySpline))
  (bind _walkspline (Variables|Default|GetWalkSpline))
  (bind _asbp_third_person_character (Utilities|Casting|CastToBP_ThirdPersonCharacter OtherActor))
  (Variables|Default|SetCharacterRef _asbp_third_person_character)
  (Utilities|FlowControl|DoOnce false
    (:Completed
      (Variables|/Game/DesertCharacter/BP_ThirdPersonCharacter.BP_ThirdPersonCharacter_C|SetBP_IllusionRef (Variables|Default|GetCharacterRef) 0)
      (Default|EndingEvent (Variables|Default|GetCharacterRef))
      (Utilities|FlowControl|Delay 2.5)
      (Input|DisableInput (Game|Player|GetPlayerPawn 0) (Game|GetPlayerController 0))
      (Game|Player|SetViewTargetwithBlend (Game|GetPlayerController 0) (Variables|Default|GetEndingIntroCam) 0.0 "VTBlend_Linear" 0.0 false)
      (Default|CameraRotation (Variables|Default|GetEndingIntroCam))
      (Utilities|FlowControl|Delay 5.0)
      (Game|Player|SetViewTargetwithBlend (Game|GetPlayerController 0) self 0.0 "VTBlend_Linear" 0.0 false)
      (Variables|Default|SetCameraActove true)
      (Collision|SetActorEnableCollision _returnvalue_2 false)
      (Components|Animation|PlayAnimation (Variables|/Script/Engine.Character|GetMesh _returnvalue_2) "/Game/DesertCharacter/Animations/AS_Walk.AS_Walk" true)
      (bind _newtrack_0 (Timeline|Timeline_1 PlayFromStart)
        (:Update
          (Transformation|SetActorLocationAndRotation _returnvalue_2 (.location (Spline|GetTransformatDistanceAlongSpline _walkspline (Math|Float|Lerp 0.0 (Spline|GetSplineLength _walkspline) (- 1.0 _newtrack_0)) "World" false)) (Math|Rotator|CombineRotators (.rotation (Spline|GetTransformatDistanceAlongSpline _walkspline (Math|Float|Lerp 0.0 (Spline|GetSplineLength _walkspline) (- 1.0 _newtrack_0)) "World" false)) "0.000000,180.000000,0.000000")))
        (:Finished
          (Components|Animation|PlayAnimation (Variables|/Script/Engine.Character|GetMesh (Game|GetPlayerCharacter 0)) "/Game/DesertCharacter/Animations/AS_Idle.AS_Idle" true)
          (Variables|Default|SetFallStartLoc (Transformation|GetActorLocation (Variables|Default|GetCharacterRef)))
          (Variables|Default|SetFallStartRot (Transformation|GetActorRotation (Variables|Default|GetCharacterRef)))
          (Utilities|FlowControl|Delay 1.0)
          (bind _newtrack_1 (Timeline|Timeline_3 Play)
            (:Update
              (Transformation|SetWorldLocationAndRotation (Variables|/Script/Engine.Character|GetCapsuleComponent (Variables|Default|GetCharacterRef)) (Math|Vector|Lerp(Vector) (Variables|Default|GetFallStartLoc) (Variables|Default|GetFallLocation) _newtrack_1) (Math|Rotator|Lerp(Rotator) (Variables|Default|GetFallStartRot) (Variables|Default|GetFallRotation) _newtrack_1) false false))
            (:Finished
              (Utilities|FlowControl|Delay 1.0)
              (bind _asbp_third_person_character_2 (Utilities|Casting|CastToBP_ThirdPersonCharacter _returnvalue))
              (Rendering|SetVisibility (Variables|/Script/Engine.Character|GetMesh _returnvalue) false false)
              (Rendering|SetVisibility (Variables|/Game/DesertCharacter/BP_ThirdPersonCharacter.BP_ThirdPersonCharacter_C|GetPers_low__2__Object001 _asbp_third_person_character_2) true false)
              (Utilities|FlowControl|Delay 1.5)
              (bind _newtrack_0_2 (Timeline|Timeline_2 PlayFromStart)
                (:Update
                  (Transformation|SetActorLocationAndRotation (Game|GetPlayerCharacter 0) (.location (Spline|GetTransformatDistanceAlongSpline _flyspline (Math|Float|Lerp 0.0 (Spline|GetSplineLength _flyspline) _newtrack_0_2) "World" false)) "0.000000,125.000000,0.000000")
                  (Variables|/Script/CinematicCamera.CineCameraComponent|SetLensSettings (Variables|Default|GetCineCamera) (Utilities|Struct|MakeCameraLensSettings (Math|Float|Lerp 25.0 35.0 _newtrack_0_2) (Math|Float|Lerp 25.0 35.0 _newtrack_0_2) 1.4 22.0 15.0 1.0 7)))
                (:Finished
                  (Utilities|FlowControl|Delay 3.0)
                  (Game|QuitGame 0 "Quit" false))))))))))

(event Custom|VisionON
  (bind _barrier (Variables|Default|GetBarrier))
  (Utilities|Array|Clear (Variables|Default|GetDissappearMaterials))
  (Utilities|Array|Clear (Variables|Default|GetAppearMaterials))
  (for _array_element (Variables|Default|GetIllusionOnAppearActors)
    (Collision|SetCollisionResponsetoAllChannels (Actor|GetComponentbyClass _array_element "/Script/Engine.StaticMeshComponent") "ECR_Block")
    (for _array_element_2 (Rendering|Material|GetMaterials (Actor|GetComponentbyClass _array_element "/Script/Engine.StaticMeshComponent"))
      (bind _returnvalue (Rendering|Material|CreateDynamicMaterialInstance (Actor|GetComponentbyClass _array_element "/Script/Engine.StaticMeshComponent") (Utilities|Array|Length (Variables|Default|GetAppearMaterials)) _array_element_2 "None" :!class /Script/Engine.PrimitiveComponent))
      (Utilities|Array|Add (Variables|Default|GetAppearMaterials) _returnvalue)))
  (for _array_element_3 (Variables|Default|GetIllusionOnDissappearActors)
    (Collision|SetCollisionResponsetoAllChannels (Actor|GetComponentbyClass _array_element_3 "/Script/Engine.StaticMeshComponent") "ECR_Ignore")
    (for _array_element_4 (Rendering|Material|GetMaterials (Actor|GetComponentbyClass _array_element_3 "/Script/Engine.StaticMeshComponent"))
      (bind _returnvalue_2 (Rendering|Material|CreateDynamicMaterialInstance (Actor|GetComponentbyClass _array_element_3 "/Script/Engine.StaticMeshComponent") (Utilities|Array|Length (Variables|Default|GetDissappearMaterials)) _array_element_4 "None" :!class /Script/Engine.PrimitiveComponent))
      (Utilities|Array|Add (Variables|Default|GetDissappearMaterials) _returnvalue_2)))
  (bind _returnvalue_3 (Rendering|Material|CreateDynamicMaterialInstance _barrier 0 (Rendering|Material|GetMaterial _barrier 0) "None" :!class /Script/Engine.PrimitiveComponent))
  (Utilities|Array|Add (Variables|Default|GetDissappearMaterials) _returnvalue_3)
  (CallFunction|MaterialAppear)
  (CallFunction|MaterialDissapear))

(event Custom|VisionOFF
  (bind _barrier (Variables|Default|GetBarrier))
  (Utilities|Array|Clear (Variables|Default|GetDissappearMaterials))
  (Utilities|Array|Clear (Variables|Default|GetAppearMaterials))
  (Utilities|FlowControl|Sequence
    (:then_0
      (for _array_element (Variables|Default|GetIllusionOffAppearActors)
        (Collision|SetCollisionResponsetoAllChannels (Actor|GetComponentbyClass _array_element "/Script/Engine.StaticMeshComponent") "ECR_Block")
        (for _array_element_2 (Rendering|Material|GetMaterials (Actor|GetComponentbyClass _array_element "/Script/Engine.StaticMeshComponent"))
          (bind _returnvalue (Rendering|Material|CreateDynamicMaterialInstance (Actor|GetComponentbyClass _array_element "/Script/Engine.StaticMeshComponent") (Utilities|Array|Length (Variables|Default|GetAppearMaterials)) _array_element_2 "None" :!class /Script/Engine.PrimitiveComponent))
          (Utilities|Array|Add (Variables|Default|GetAppearMaterials) _returnvalue)))
      (for _array_element_3 (Variables|Default|GetIllusionOffDissappearActors)
        (Collision|SetCollisionResponsetoAllChannels (Actor|GetComponentbyClass _array_element_3 "/Script/Engine.StaticMeshComponent") "ECR_Ignore")
        (for _array_element_4 (Rendering|Material|GetMaterials (Actor|GetComponentbyClass _array_element_3 "/Script/Engine.StaticMeshComponent"))
          (bind _returnvalue_2 (Rendering|Material|CreateDynamicMaterialInstance (Actor|GetComponentbyClass _array_element_3 "/Script/Engine.StaticMeshComponent") (Utilities|Array|Length (Variables|Default|GetDissappearMaterials)) _array_element_4 "None" :!class /Script/Engine.PrimitiveComponent))
          (Utilities|Array|Add (Variables|Default|GetDissappearMaterials) _returnvalue_2))))
    (:then_1
      (bind _returnvalue_3 (Rendering|Material|CreateDynamicMaterialInstance _barrier 0 (Rendering|Material|GetMaterial _barrier 0) "None" :!class /Script/Engine.PrimitiveComponent))
      (Utilities|Array|Add (Variables|Default|GetAppearMaterials) _returnvalue_3)
      (CallFunction|MaterialAppear)
      (CallFunction|MaterialDissapear))))

(event Custom|MaterialDissapear
  (bind (_direction _newtrack_0 _newtrack_2) (Timeline|Timeline PlayFromStart)
    (:Update
      (for _array_element (Variables|Default|GetDissappearMaterials)
        (Rendering|Material|SetScalarParameterValue _array_element "AppearanceBlend" _newtrack_0 :!class /Script/Engine.MaterialInstanceDynamic)
        (Rendering|Material|SetScalarParameterValue _array_element "Emissive_Mult" _newtrack_2 :!class /Script/Engine.MaterialInstanceDynamic)))))

(event Custom|MaterialAppear
  (bind (_direction _newtrack_0 _newtrack_1) (Timeline|Timeline_0 PlayFromStart)
    (:Update
      (for _array_element (Variables|Default|GetAppearMaterials)
        (Rendering|Material|SetScalarParameterValue _array_element "AppearanceBlend" _newtrack_0 :!class /Script/Engine.MaterialInstanceDynamic)
        (Rendering|Material|SetScalarParameterValue _array_element "Emissive_Mult" _newtrack_1 :!class /Script/Engine.MaterialInstanceDynamic)))))

(event Custom|TestLastScene
  (bind _returnvalue (Game|GetPlayerCharacter 0))
  (bind _returnvalue_2 (Game|GetPlayerCharacter 0))
  (bind _characterref (Variables|Default|GetCharacterRef))
  (bind _flyspline (Variables|Default|GetFlySpline))
  (bind _walkspline (Variables|Default|GetWalkSpline))
  (bind _characterref_2 (Variables|Default|GetCharacterRef))
  (Utilities|FlowControl|DoOnce false
    (:Completed
      (Variables|/Game/DesertCharacter/BP_ThirdPersonCharacter.BP_ThirdPersonCharacter_C|SetBP_IllusionRef _characterref 0)
      (Default|EndingEvent _characterref)
      (Utilities|FlowControl|Delay 2.5)
      (Input|DisableInput (Game|Player|GetPlayerPawn 0) (Game|GetPlayerController 0))
      (Game|Player|SetViewTargetwithBlend (Game|GetPlayerController 0) (Variables|Default|GetEndingIntroCam) 0.0 "VTBlend_Linear" 0.0 false)
      (Default|CameraRotation (Variables|Default|GetEndingIntroCam))
      (Utilities|FlowControl|Delay 5.0)
      (Game|Player|SetViewTargetwithBlend (Game|GetPlayerController 0) self 0.0 "VTBlend_Linear" 0.0 false)
      (Variables|Default|SetCameraActove true)
      (Collision|SetActorEnableCollision _returnvalue_2 false)
      (Components|Animation|PlayAnimation (Variables|/Script/Engine.Character|GetMesh _returnvalue_2) "/Game/DesertCharacter/Animations/AS_Walk.AS_Walk" true)
      (bind _newtrack_0 (Timeline|Timeline_1 PlayFromStart)
        (:Update
          (Transformation|SetActorLocationAndRotation _returnvalue_2 (.location (Spline|GetTransformatDistanceAlongSpline _walkspline (Math|Float|Lerp 0.0 (Spline|GetSplineLength _walkspline) (- 1.0 _newtrack_0)) "World" false)) (Math|Rotator|CombineRotators (.rotation (Spline|GetTransformatDistanceAlongSpline _walkspline (Math|Float|Lerp 0.0 (Spline|GetSplineLength _walkspline) (- 1.0 _newtrack_0)) "World" false)) "0.000000,180.000000,0.000000")))
        (:Finished
          (Components|Animation|PlayAnimation (Variables|/Script/Engine.Character|GetMesh (Game|GetPlayerCharacter 0)) "/Game/DesertCharacter/Animations/AS_Idle.AS_Idle" true)
          (Variables|Default|SetFallStartLoc (Transformation|GetActorLocation _characterref_2))
          (Variables|Default|SetFallStartRot (Transformation|GetActorRotation _characterref_2))
          (Utilities|FlowControl|Delay 1.0)
          (bind _newtrack_1 (Timeline|Timeline_3 Play)
            (:Update
              (Transformation|SetWorldLocationAndRotation (Variables|/Script/Engine.Character|GetCapsuleComponent (Variables|Default|GetCharacterRef)) (Math|Vector|Lerp(Vector) (Variables|Default|GetFallStartLoc) (Variables|Default|GetFallLocation) _newtrack_1) (Math|Rotator|Lerp(Rotator) (Variables|Default|GetFallStartRot) (Variables|Default|GetFallRotation) _newtrack_1) false false))
            (:Finished
              (Utilities|FlowControl|Delay 1.0)
              (bind _asbp_third_person_character (Utilities|Casting|CastToBP_ThirdPersonCharacter _returnvalue))
              (Rendering|SetVisibility (Variables|/Script/Engine.Character|GetMesh _returnvalue) false false)
              (Rendering|SetVisibility (Variables|/Game/DesertCharacter/BP_ThirdPersonCharacter.BP_ThirdPersonCharacter_C|GetPers_low__2__Object001 _asbp_third_person_character) true false)
              (Utilities|FlowControl|Delay 1.5)
              (bind _newtrack_0_2 (Timeline|Timeline_2 PlayFromStart)
                (:Update
                  (Transformation|SetActorLocationAndRotation (Game|GetPlayerCharacter 0) (.location (Spline|GetTransformatDistanceAlongSpline _flyspline (Math|Float|Lerp 0.0 (Spline|GetSplineLength _flyspline) _newtrack_0_2) "World" false)) "0.000000,125.000000,0.000000")
                  (Variables|/Script/CinematicCamera.CineCameraComponent|SetLensSettings (Variables|Default|GetCineCamera) (Utilities|Struct|MakeCameraLensSettings (Math|Float|Lerp 25.0 35.0 _newtrack_0_2) (Math|Float|Lerp 25.0 35.0 _newtrack_0_2) 1.4 22.0 15.0 1.0 7)))
                (:Finished
                  (Utilities|FlowControl|Delay 3.0)
                  (Game|QuitGame 0 "Quit" false))))))))))

(event EventTick
  (params (DeltaSeconds :type Float%20%28single-precision%29))
  (if (Variables|Default|GetCameraActove)
    (Transformation|SetWorldRotation (Variables|Default|GetCineCamera) (Math|Rotator|FindLookatRotation (Transformation|GetWorldLocation (Variables|Default|GetCineCamera)) (+ (Transformation|GetActorLocation (Game|Player|GetPlayerPawn 0)) "0.000000,0.000000,60.000000")) false false)))

(event EventBeginPlay
  (bind _returnvalue (Actor|GetActorOfClass "/Game/DesertCharacter/BP_ThirdPersonCharacter.BP_ThirdPersonCharacter_C"))
  (bind _output_get (Variables|Default|SetCharacterRef _returnvalue))
  (Components|Timeline|SetPlayRate (Variables|Default|GetTimeline) (Variables|/Game/DesertCharacter/BP_ThirdPersonCharacter.BP_ThirdPersonCharacter_C|GetTimelinePlayrates _output_get))
  (bind _returnvalue_2 (Actor|GetActorOfClass "/Game/BP_EndingIntroCamera.BP_EndingIntroCamera_C"))
  (Variables|Default|SetEndingIntroCam _returnvalue_2))

(fn ConstructionScript)